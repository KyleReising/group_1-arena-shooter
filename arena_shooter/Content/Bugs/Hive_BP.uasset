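; Bug hive actor that the player can destroy with a bomb once none of its bugs remain.
; It tallies owned bugs and shows that count on a widget while the player's ToggleCone overlaps its pylon.
; Tick relocates an activated hive to a random reachable point when nearby bugs stay away past a timer, if respawning is allowed.
; Planting flags destruction; Tick then spawns an actor, deregisters from the brood spawner and updates player numbers.
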(event `self.ReceiveBeginPlay`
  (bind _asmy_hive_ui (cast `/Game/UI/MyHiveUI` (`WidgetComponent.GetUserWidgetObject` (`self.Widget`))))
  (bind _output_get (set `self.As My Hive UI` _asmy_hive_ui))
  (`Widget.SetVisibility` _output_get "Hidden")
  (bind _returnvalue (`GameplayStatics.GetActorOfClass` "/Game/Bugs/Brood_Spawner_BP.Brood_Spawner_BP_C"))
  (set `self.Reference Brood Spawner` _returnvalue)
  (bind _returnvalue_2 (`GameplayStatics.GetActorOfClass` "/Game/Player/MyPlayer.MyPlayer_C"))
  (set `self.As My Player` _returnvalue_2))

(event `self.ReceiveTick`
  (params (DeltaSeconds :type "Float (single-precision)"))
  (set `self.Delta Seconds` DeltaSeconds)
  (`self.Bug Number Get`)
  (`self.DestroySelfCheck`)
  ;[1 1 1] Update UI.
  (set `/Game/UI/MyHiveUI.BugsLeft` (`self.Bugs Owned`) (`self.As My Hive UI`))
  ;[1 1 1] If we have activated, and all of our bugs ran away, wait some time incase one comes back, and respawn if not
  (if (and (`self.Activated`) (<= (`self.Num_Bugs_Near`) 0))
    ;[1 1 1] Check to see if our timer has counted down
    (if (and (<= (`self.cur_respawn_timer`) 0.0) (`self.allow_respawning`))
      ;[1 1 1] Our timer has counted down, reposition our hive and deactive it
      (`self.K2_SetActorLocation` (`NavigationSystemV1.K2_GetRandomReachablePointInRadius` (`SceneComponent.K2_GetComponentLocation` (`self.Bug_collider`)) 1000000.0 null null))
      (set `self.Activated` false)
      (else
        ;[1 1 1] Our timer has not counted down, continue to countdown
        (set `self.cur_respawn_timer` (- (`self.cur_respawn_timer`) (`self.Delta Seconds`)))))))

(event `self.pylon.OnComponentBeginOverlap`
  (params (OverlappedComponent :type "PrimitiveComponent Object Reference") (OtherActor :type "Actor Object Reference") (OtherComp :type "PrimitiveComponent Object Reference") (OtherBodyIndex :type Integer) (bFromSweep :type Boolean) (SweepResult :type "HitResult Structure (by ref)"))
  (if (`self.ActorHasTag` OtherActor "Player")
    (if (`ActorComponent.ComponentHasTag` OtherComp "ToggleCone")
      (`Widget.SetVisibility` (`self.As My Hive UI`) "Visible")
      (set `self.Hive Looked At` self)
      (`self.Bomb Check`))))

(event `self.pylon.OnComponentEndOverlap`
  (params (OverlappedComponent :type "PrimitiveComponent Object Reference") (OtherActor :type "Actor Object Reference") (OtherComp :type "PrimitiveComponent Object Reference") (OtherBodyIndex :type Integer))
  (if (`self.ActorHasTag` OtherActor "Player")
    (if (`ActorComponent.ComponentHasTag` OtherComp "ToggleCone")
      (`Widget.SetVisibility` (`self.As My Hive UI`) "Hidden")
      (set `self.Hive Looked At` null)
      (`self.Bomb Check`))))

(fn `Bomb Check`
  (bind _as_my_hive_ui (`self.As My Hive UI`))
  (bind _bombs_ (`/Game/Player/MyPlayer.BombsCheck` (`self.As My Player`)))
  (if (and _bombs_ (== (`self.Bugs Owned`) 0))
    (set `/Game/UI/MyHiveUI.Action Text` (`self.Bomb Plant Text`) _as_my_hive_ui)
    (set `self.Bomb Can Plant?` true)
    (else
      (set `/Game/UI/MyHiveUI.Action Text` "" _as_my_hive_ui)
      (set `self.Bomb Can Plant?` false))))

(fn `Bomb Plant`
  (returns (`Hive to Remove from Array` :type "/Game/Bugs/Hive_BP Object Reference"))
  (bind _as_my_player (`self.As My Player`))
  (`self.Bomb Check`)
  (if (and (== (`self.Hive Looked At`) self) (`self.Bomb Can Plant?`))
    (set `/Game/Player/MyPlayer.Number Of Bombs` (- (`/Game/Player/MyPlayer.Number Of Bombs` _as_my_player) 1) _as_my_player)
    (set `self.Destroy Self` true)
    (return self)))

(fn `Bug Number Get`
  ;[1 1 1] Get number of bugs in this hive. Calls ONCE per Check for Bugs == True.
  (if (`self.Check For Bugs`)
    (bind _outactors (`GameplayStatics.GetAllActorsOfClass` "/Game/Bugs/Bug_Pawn_BP.Bug_Pawn_BP_C"))
    (for _array_element _outactors
      (if (== (`/Game/Bugs/Bug_Pawn_BP.My_hive` _array_element) self)
        (bind _output_get (set `self.Bugs Owned` (+ (`self.Bugs Owned`) 1)))))
    (set `self.Check For Bugs` false)))

(fn `Bug Number Remove`
  (set `self.Bugs Owned` (- (`self.Bugs Owned`) 1)))

(fn `DestroySelfCheck`
  (if (`self.Destroy Self`)
    (set `self.Hive Looked At` null)
    (`|SpawnActorFromClass` "/Game/Bugs/HiveDestroy/MyHiveDestroy.MyHiveDestroy_C" (`SceneComponent.K2_GetComponentToWorld` (`self.hive`)) "Undefined" "OverrideRootScale" null null)
    (`KismetArrayLibrary.Array_RemoveItem` (`/Game/Bugs/Brood_Spawner_BP.my_hives` (`self.Reference Brood Spawner`)) self)
    (bind _returnvalue (`GameplayStatics.GetActorOfClass` "/Game/Player/MyPlayer.MyPlayer_C"))
    (`/Game/Player/MyPlayer.NumbersUpdate` _returnvalue 100)
    (`self.K2_DestroyActor`)))

(fn `Do Bug Enter`
  (params (`Within Hive` :type Boolean))
  (if (not `Within Hive`)
    (set `self.Num_Bugs_Near` (+ (`self.Num_Bugs_Near`) 1))
    (set `self.Activated` true)))

(fn `Do Bug Exit`
  (params (`Within Hive` :type Boolean))
  (if `Within Hive`
    (set `self.Num_Bugs_Near` (- (`self.Num_Bugs_Near`) 1))
    (if (<= (`self.Num_Bugs_Near`) 0)
      (set `self.cur_respawn_timer` (`self.base_respawn_timer`)))))

(fn `UserConstructionScript`)
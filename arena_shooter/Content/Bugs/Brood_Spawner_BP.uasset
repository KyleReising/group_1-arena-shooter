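; Brood spawner actor that populates the level with bug hives and their bugs on BeginPlay, and can delete the whole brood.
; Hives spawn at random reachable navmesh points around the spawner, then bugs spawn near hives round-robin, each linked to its hive and checked for hive collisions.
; A difficulty function scales hive and bug counts and enables hive respawning at higher levels, affecting later spawns.
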(event `self.ReceiveBeginPlay`
  (`self.do_spawn_brood`))

(fn `do_delete_brood`
  (locals (temp_integer_variable :type Integer))
  (for _array_element (`self.my_bugs`)
    (`self.K2_DestroyActor` _array_element))
  (`KismetArrayLibrary.Array_Clear` (`self.my_bugs`))
  (for _array_element_2 (`self.my_hives`)
    (`self.K2_DestroyActor` _array_element_2))
  (`KismetArrayLibrary.Array_Clear` (`self.my_hives`)))

(fn `do_increase_difficulty_level`
  (params (`Difficulty increase` :type Integer :default 1))
  (locals (hive_multiplier_modifier :type Integer :default 1) (bug_per_hive_multiplier_modifier :type Integer :default 3) (minimum_hives :type Integer :default 1))
  ;[1 1 1] Increase difficulty
  (set `self.difficulty_level` (+ (`self.difficulty_level`) `Difficulty increase`))
  ;[1 1 1] Difficulty >= 4 means hives are allowed to respawn
  (if (>= (`self.difficulty_level`) 4)
    (set `self.allow_hive_respawning` true))
  ;[1 1 1] Update number of hive: Difficulty mod * Hive multipier + minimum hives
  (bind _output_get (set `self.num_of_hives` (+ (* (`local.hive_multiplier_modifier`) (`self.difficulty_level`)) (`local.minimum_hives`))))
  ;[1 1 1] Update number of bugs: Difficulty mod * Bugs/Hive * number of hives
  (set `self.num_of_bugs` (* _output_get (`self.difficulty_level`) (`local.bug_per_hive_multiplier_modifier`))))

(fn `do_spawn_brood`
  (locals (temp_range_integer_variable :type Integer :default 0) (temp_hive_assigning_variable :type Integer))
  (bind _randomlocation (`NavigationSystemV1.K2_GetRandomReachablePointInRadius` (`self.K2_GetActorLocation`) 100000.0 null null))
  (bind _randomlocation_2 (`NavigationSystemV1.K2_GetRandomReachablePointInRadius` (`self.K2_GetActorLocation` (`|GetArrayItem` (`self.my_hives`) (`local.temp_hive_assigning_variable`))) 600.0 null null))
  ;[1 1 1] Creating our hives and adding them to our "my_hives" array
  (set `local.temp_range_integer_variable` 0)
  (while (< (`local.temp_range_integer_variable`) (`self.num_of_hives`))
    (bind _returnvalue (`|SpawnActorFromClass` "/Game/Bugs/Hive_BP.Hive_BP_C" (`KismetMathLibrary.MakeTransform` (`KismetMathLibrary.MakeVector` (.x _randomlocation) (.y _randomlocation) 20.0) (struct) (6.0 6.0 6.0)) "AdjustIfPossibleButAlwaysSpawn" "OverrideRootScale" null null))
    (`KismetArrayLibrary.Array_Add` (`self.my_hives`) _returnvalue)
    (set `local.temp_range_integer_variable` (+ (`local.temp_range_integer_variable`) 1))
    (set `/Game/Bugs/Hive_BP.allow_respawning` (`self.allow_hive_respawning`) _returnvalue))
  (`KismetSystemLibrary.PrintString` "Finished spawning Hives")
  ;[1 1 1] Creating our bugs, adding them to our "my_bugs" array, and assigning them to a hive
  (set `local.temp_range_integer_variable` 0)
  (while (< (`local.temp_range_integer_variable`) (`self.num_of_bugs`))
    (bind _returnvalue_2 (`|SpawnActorFromClass` "/Game/Bugs/Bug_Pawn_BP.Bug_Pawn_BP_C" (`KismetMathLibrary.MakeTransform` (`KismetMathLibrary.MakeVector` (.x _randomlocation_2) (.y _randomlocation_2) 35.0) (struct) (0.3 0.3 0.3)) "AdjustIfPossibleButDontSpawnIfColliding" "OverrideRootScale" null null))
    (`KismetArrayLibrary.Array_Add` (`self.my_bugs`) _returnvalue_2)
    (set `/Game/Bugs/Bug_Pawn_BP.My_hive` (`|GetArrayItem` (`self.my_hives`) (`local.temp_hive_assigning_variable`)) _returnvalue_2)
    (`/Game/Bugs/Bug_Pawn_BP.do_check_colliding_with_hives` _returnvalue_2)
    (set `local.temp_range_integer_variable` (+ (`local.temp_range_integer_variable`) 1))
    (bind _output_get (set `local.temp_hive_assigning_variable` (+ (`local.temp_hive_assigning_variable`) 1)))
    (if (>= _output_get (`self.num_of_hives`))
      (set `local.temp_hive_assigning_variable` 0)))
  (`KismetSystemLibrary.PrintString` "Finished spawning Bugs"))

(fn `UserConstructionScript`)